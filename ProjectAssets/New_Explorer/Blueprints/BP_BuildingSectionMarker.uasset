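; BP_BuildingSectionMarker is a POI marker for a building that reveals that building's floor section markers when selected.
; On BeginPlay it puts a floor icon widget, filled from its floor value, into its widget component.
; Selection loops the GameInstance's POIs, showing floor markers with a matching building and hiding other buildings' markers.
; It then resets the player controller's section view and stores the current building, calling functions and setting variables by name.
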(event EventBeginPlay
  (bind _self self)
  (Class|LanessaV2Widget|CallParentFunction self "ReceiveBeginPlay")
  (bind _returnvalue (UserInterface|CreateWidget "/Game/New_Explorer/Blueprints/Widgets/BP_3D_Widget_FloorIcon.BP_3D_Widget_FloorIcon_C"))
  (Variables|/Game/New_Explorer/Blueprints/Widgets/BP_3D_Widget_FloorIcon.BP_3D_Widget_FloorIcon_C|SetOwningPOI _returnvalue _self)
  (bind _outfloor (Class|LanessaV2Widget|GetOwnFloorandBuilding _self))
  (Default|SetValues _returnvalue _outfloor)
  (UserInterface|SetWidget (Variables|Default|GetWidgetComponent) _returnvalue))

(event Collision|EventActorBeginOverlap
  (params (OtherActor :type Actor%20Object%20Reference)))

(event EventTick
  (params (DeltaSeconds :type Float%20%28single-precision%29))
  (|CallParentFunction DeltaSeconds))

(event EventSelectPOI
  (Class|LanessaV2Widget|CallParentFunction self "Select_POI")
  (Development|PrintString "BUILDING-DEBUG: Select_POI fired")
  (bind _outbuilding (Class|LanessaV2Widget|GetOwnFloorandBuilding self))
  (bind _asbp_explorer_game_instance_ln (Utilities|Casting|CastToBP_Explorer_GameInstance_LN (Game|GetGameInstance)))
  (for _array_element (Variables|/Game/New_Explorer/Blueprints/BP_Explorer_GameInstance_LN.BP_Explorer_GameInstance_LN_C|GetBP_POIs _asbp_explorer_game_instance_ln)
    (bind _asbp_floor_section_marker (Utilities|Casting|CastToBP_FloorSectionMarker _array_element))
    (bind _outbuilding_2 (Class|LanessaV2Widget|GetOwnFloorandBuilding _asbp_floor_section_marker))
    (if (Utilities|Enum|Equal(Enum) _outbuilding_2 _outbuilding)
      (Class|LanessaV2Widget|CallPOIShowHide _asbp_floor_section_marker true)
      (else
        (Class|LanessaV2Widget|CallPOIShowHide _asbp_floor_section_marker false))))
  (bind _asbp_explorer_pc (Utilities|Casting|CastToBP_Explorer_PC (Game|GetPlayerController 0)))
  (Class|LanessaV2Widget|CallActorFunction _asbp_explorer_pc "Reset_SectionView")
  (Class|LanessaV2Widget|SetActorStringVariable _asbp_explorer_pc "CurrentQirqimBuilding" _outbuilding))

(fn ConstructionScript
  (|CallParentFunction))