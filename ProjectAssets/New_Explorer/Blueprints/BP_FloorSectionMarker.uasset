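; Floor marker POI that, when selected, switches the explorer to a sectioned view of its floor.
; BeginPlay fills its widget component with a floor icon showing its floor number.
; Selection, given a valid SectionViewVolume, shows type-2 POIs matching its floor and building via a DataTable and hides markers of higher floors.
; It then passes the volume's bounds and normalized yaw to the player controller's section mask and records the current building.
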(event Custom|OnFloorMarkerSelected
  (bind _sectionview_volume (Variables|Default|GetSectionView_Volume))
  (bind (_origin _boxextent) (Collision|GetActorBounds _sectionview_volume false false))
  (Development|PrintString "DEBUG: OnFloorMarkerSelected body running")
  (Utilities|IsValid _sectionview_volume
    (:Is%20Valid
      (bind (_outfloor _outbuilding) (Class|LanessaV2Widget|GetOwnFloorandBuilding self))
      (for _array_element (Variables|/Game/New_Explorer/Blueprints/BP_Explorer_GameInstance_LN.BP_Explorer_GameInstance_LN_C|GetBP_POIs (Variables|Default|GetBP_Explorer_GI))
        (Utilities|FlowControl|Sequence
          (:then_0
            (bind _returnvalue (Class|LanessaV2Widget|GetPOITypeasInt _array_element))
            (if (== _returnvalue (Class|KismetSystemLibrary|MakeLiteralInteger 2))
              (bind _returnvalue_2 (Class|LanessaV2Widget|DoesPOIMatchFloorBuilding _array_element "/Game/New_Explorer/Blueprints/DataTables/DT_Demonstration_01_POI_Filter.DT_Demonstration_01_POI_Filter" _outfloor _outbuilding))
              (if _returnvalue_2
                (Class|LanessaV2Widget|CallPOIShowHide _array_element true)
                (else
                  (Class|LanessaV2Widget|CallPOIShowHide _array_element false)))))
          (:then_1
            (bind _asbp_floor_section_marker (Utilities|Casting|CastToBP_FloorSectionMarker _array_element))
            (bind _outfloor_2 (Class|LanessaV2Widget|GetOwnFloorandBuilding _asbp_floor_section_marker))
            (if (> _outfloor_2 _outfloor)
              (Class|LanessaV2Widget|CallPOIShowHide _array_element false)
              (else
                (Class|LanessaV2Widget|CallPOIShowHide _array_element true))))))
      (bind _asbp_explorer_pc (Utilities|Casting|CastToBP_Explorer_PC (Game|GetPlayerController 0))
        (:then
          (Utilities|FlowControl|Sequence
            (:then_0
              (Default|SectionViewMask _asbp_explorer_pc (Math|Conversions|ToLinearColor(Vector) _origin) (Math|Conversions|ToLinearColor(Vector) (* _boxextent (Math|Float|MakeLiteralFloat 2.0))) (/ (Class|KismetMathLibrary|ClampAxis (.Yaw (Math|Rotator|BreakRotator (Transformation|GetActorRotation _sectionview_volume)))) (Math|Float|MakeLiteralFloat 3.6e+02)))
              (Development|PrintString "DEBUG: SectionView_Mask call completed"))
            (:then_1
              (Variables|/Game/New_Explorer/Blueprints/BP_Explorer_PC.BP_Explorer_PC_C|SetCurrentQirqimBuilding _asbp_explorer_pc _outbuilding))))
        (:CastFailed
          (Development|PrintString "DEBUG: CastToBP_Explorer_PC FAILED"))))))

(event Custom|OnFloorIconBeginPlay
  (bind _self self)
  (bind _returnvalue (UserInterface|CreateWidget "/Game/New_Explorer/Blueprints/Widgets/BP_3D_Widget_FloorIcon.BP_3D_Widget_FloorIcon_C"))
  (Variables|/Game/New_Explorer/Blueprints/Widgets/BP_3D_Widget_FloorIcon.BP_3D_Widget_FloorIcon_C|SetOwningPOI _returnvalue _self)
  (bind _outfloor (Class|LanessaV2Widget|GetOwnFloorandBuilding _self))
  (Default|SetValues _returnvalue _outfloor)
  (UserInterface|SetWidget (Variables|Default|GetWidgetComponent) _returnvalue))

(event EventBeginPlay
  (|CallParentFunction)
  (CallFunction|OnFloorIconBeginPlay))

(event Collision|EventActorBeginOverlap
  (params (OtherActor :type Actor%20Object%20Reference)))

(event EventTick
  (params (DeltaSeconds :type Float%20%28single-precision%29))
  (|CallParentFunction DeltaSeconds))

(event EventSelectPOI
  (Class|LanessaV2Widget|CallParentFunction self "Select_POI")
  (Development|PrintString "DEBUG: Select_POI fired on FloorSectionMarker")
  (CallFunction|OnFloorMarkerSelected))

(fn ConstructionScript
  (|CallParentFunction))